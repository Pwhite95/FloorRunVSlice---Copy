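; BP_Slot_Atom is a slot Blueprint for atoms in the VRAssembling content, configured by an atomic number.
; Its construction script sets a sphere as the hologram mesh, scaled uniformly by atomic number with a lower limit.
; It builds a single slot name from "Atom" plus that number, then runs the parent construction script.
; The event graph holds only disabled placeholder events.
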(event EventBeginPlay
  (|CallParentFunction) ; This node is disabled and will not be called.\nDrag off pins to build functionality.
)

(event Collision|EventActorBeginOverlap
  (params (OtherActor :type Actor%20Object%20Reference)))

(event EventTick
  (params (DeltaSeconds :type Float%20%28single-precision%29)))

(fn ConstructionScript
  (Variables|Default|SetHoloMesh "/Game/VRAssembling/Meshes/SM_Sphere.SM_Sphere")
  (Variables|Default|SetHoloTransform (Math|Transform|MakeTransform "0, 0, 0" "0, 0, 0" (Math|Conversions|ToVector(Float) (/ (Math|Float|Max(Float) (Math|Conversions|ToFloat(Integer) (Variables|Default|GetAtomicNumber)) 4.0) 5e+01))))
  (Variables|Default|SetSlots (Utilities|Array|MakeArray (Utilities|String|Append "Atom" (Utilities|String|ToString(Integer) (Variables|Default|GetAtomicNumber)))))
  (|CallParentFunction))