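; Grabbable static-mesh part for VR assembly that a motion controller can force-pull, pick up, drop and snap into a slot.
; Construction applies the configured mesh and physics setting, which Drop restores on release.
; Attach has the pawn release any held part, then disables physics and snaps it to the slot.
; Pickup refuses blocked or locked slots, otherwise frees the slot; Touch forwards velocity to push-type holo slots.
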(event EventPull
  (params (Controller :type BP%20Motion%20Controller%20Object%20Reference))
  (if (not (Variables|Default|GetAttached))
    (if (Variables|Settings|GetForceGrabbable)
      (CallFunction|BasicPullForce (Variables|Default|GetStaticMesh) (Transformation|GetWorldLocation (Variables|/Game/VRAssembling/Blueprints/BP_MotionController.BP_MotionController_C|GetGrabSphere Controller)) 1e+03))))

(event EventTouch
  (params (Vel :type Vector :default "0, 0, 0"))
  (bind _asbp_slot_holo_push (Utilities|Casting|CastToBP_Slot_Holo_Push (Variables|Default|GetSlotActor)))
  (Default|Touch _asbp_slot_holo_push Vel))

(event EventDrop
  (Transformation|DetachFromActor "KeepWorld" "KeepWorld" "KeepWorld")
  (Physics|SetSimulatePhysics (Variables|Default|GetStaticMesh) (Variables|Settings|GetSimulatePhysics))
  (Variables|Default|SetAttached false)
  (Variables|Default|SetSlotActor 0))

(event EventAttach
  (params (Slot :type BP%20Slot%20Base%20Object%20Reference))
  (Variables|Default|SetSlotActor Slot)
  (Variables|Default|SetAttached true)
  (Utilities|FlowControl|Sequence
    (:then_0
      (Utilities|IsValid (Actor|GetAttachParentActor)
        (:Is%20Valid
          (bind _asbp_motion_controller_pawn (Utilities|Casting|CastToBP_MotionControllerPawn (Game|Player|GetPlayerPawn 0)))
          (Default|DropHolo _asbp_motion_controller_pawn self))))
    (:then_1
      (Physics|SetSimulatePhysics (Variables|Default|GetStaticMesh) false)
      (Transformation|AttachActorToActor (Variables|Default|GetSlotActor) "None" "SnapToTarget" "SnapToTarget" "KeepWorld" false))))

(fn ConstructionScript
  (Components|StaticMesh|SetStaticMesh (Variables|Default|GetStaticMesh) (Variables|Settings|GetMesh))
  (Physics|SetSimulatePhysics (Variables|Default|GetStaticMesh) (Variables|Settings|GetSimulatePhysics)))

(fn GetSlots
  (return (Utilities|Array|MakeArray (Variables|Settings|GetSlot))))

(fn IsAttached
  (return (Variables|Default|GetAttached)))

(fn Pickup
  (params (AttachTo :type Scene%20Component%20Object%20Reference) (Hand :type BP%20Motion%20Controller%20Object%20Reference))
  (Utilities|IsValid (Variables|Default|GetSlotActor)
    (:Is%20Valid
      (if (or (Default|IsBlocked (Variables|Default|GetSlotActor)) (Variables|/Game/VRAssembling/Blueprints/BP_Slot_Base.BP_Slot_Base_C|GetLockPart (Variables|Default|GetSlotActor)))
        (return false)
        (else
          _)))
    (:Is%20Not%20Valid
      _))
  (Physics|SetSimulatePhysics (Variables|Default|GetStaticMesh) false)
  (Default|HandlePickup Hand self (Variables|Pickup|GetPickupSnap) (Variables|Pickup|GetPickupSocket))
  (Utilities|IsValid (Variables|Default|GetSlotActor)
    (:Is%20Valid
      (Default|Detach (Variables|Default|GetSlotActor))
      (Variables|Default|SetSlotActor 0)
      (Variables|Default|SetAttached false)
      (return true))
    (:Is%20Not%20Valid
      (return true))))