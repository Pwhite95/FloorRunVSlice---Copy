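; Base VR assembly slot that attaches parts entering its collision sphere.
; Unattached BI_Attach parts snap in when slot types match, required slots are filled and reverse-required slots are empty; an optional InitPart starts attached.
; Slots register with their prerequisites for direct change messages, avoiding dispatchers that are buggy with subclasses, and can drop unlocked parts when requirements fail.
; Event listeners receive attach/detach messages; blocker queries exist but do not gate attachment here.
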(event OnComponentBeginOverlap(Sphere)
  (params (OverlappedComponent :type Primitive%20Component%20Object%20Reference) (OtherActor :type Actor%20Object%20Reference) (OtherComp :type Primitive%20Component%20Object%20Reference) (OtherBodyIndex :type Integer) (bFromSweep :type Boolean) (SweepResult :type Hit%20Result%20Structure%20%28by%20ref%29))
  (CallFunction|AttachTest OtherActor))

(event Custom|Detach
  (Variables|Default|SetAttachedActor 0)
  (Variables|Default|SetAttached false)
  (for _array_element (Variables|Events|GetEventListeners)
    (Class|BIEvent|Detached(Message) _array_element self))
  (for _array_element_2 (Variables|Default|GetSubMessage)
    (CallFunction|SubDetached _array_element_2 self)))

(event Custom|RegisterSub
  (params (Slot :type BP%20Slot%20Base%20Object%20Reference%20%28by%20ref%29))
  ;[1 1 1] Sending messages to subclasses because event dispatchers are buggy with subclasses
  (Utilities|Array|Add (Variables|Default|GetSubMessage) Slot))

(event Custom|SubAttached
  (params (Slot :type BP%20Slot%20Base%20Object%20Reference))
  ;[1 1 1] Sending messages to subclasses because event dispatchers are buggy with subclasses
  (if (not (CallFunction|CheckRequiredSlots))
    (if (Math|Boolean|ANDBoolean (Variables|Default|GetAttached) (Variables|Settings|GetDropPartOnLosingRequired) (not (Variables|Settings|GetLockPart)))
      (Class|BIPickup|Drop(Message) (Variables|Default|GetAttachedActor))
      (CallFunction|Detach))))

(event Custom|SubDetached
  (params (Slot :type BP%20Slot%20Base%20Object%20Reference))
  ;[1 1 1] Sending messages to subclasses because event dispatchers are buggy with subclasses
  (if (not (CallFunction|CheckRequiredSlots))
    (if (Math|Boolean|ANDBoolean (Variables|Default|GetAttached) (Variables|Settings|GetDropPartOnLosingRequired) (not (Variables|Settings|GetLockPart)))
      (Class|BIPickup|Drop(Message) (Variables|Default|GetAttachedActor))
      (CallFunction|Detach))))

(event Custom|AttachTest
  (params (Target :type Actor%20Object%20Reference))
  (if (not (Variables|Default|GetAttached))
    (if (Utilities|DoesObjectImplementInterface Target "/Game/VRAssembling/Blueprints/BI_Attach.BI_Attach_C")
      (bind _attached (Class|BIAttach|IsAttached(Message) Target))
      (Development|PrintString (Utilities|String|ToString(Boolean) _attached))
      (if (not _attached)
        (bind _slots (Class|BIAttach|GetSlots(Message) Target))
        (bind _match (CallFunction|SlotMatch _slots))
        (if (and (CallFunction|CheckRequiredSlots) _match)
          (CallFunction|Attach Target))))))

(event Custom|Attach
  (params (AttachedActor :type Actor%20Object%20Reference))
  (Variables|Default|SetAttachedActor AttachedActor)
  (Variables|Default|SetAttached true)
  (Utilities|FlowControl|Sequence
    (:then_0
      (Class|BIAttach|Attach(Message) (Variables|Default|GetAttachedActor) self))
    (:then_1
      (for _array_element (Variables|Events|GetEventListeners)
        (Class|BIEvent|Attached(Message) _array_element self))
      (for _array_element_2 (Variables|Default|GetSubMessage)
        (CallFunction|SubAttached _array_element_2 self)))))

(event EventBeginPlay
  ;[1 1 1] Sending messages to subclasses because event dispatchers are buggy with subclasses
  (Utilities|FlowControl|Sequence
    (:then_0
      (Utilities|IsValid (Variables|Initial|GetInitPart)
        (:Is%20Valid
          (CallFunction|InitialAttach))))
    (:then_1
      (for _array_element (Variables|Requirements|GetRequiredSlots)
        (CallFunction|RegisterSub _array_element self))
      (for _array_element_2 (Variables|Requirements|GetReverseRequiredSlots)
        (CallFunction|RegisterSub _array_element_2 self)))))

(fn ConstructionScript
  (Utilities|FlowControl|Sequence
    (:then_0
      (Components|Sphere|SetSphereRadius (Variables|Default|GetSphere) (Variables|Settings|GetCollisionRadius) true))
    (:then_1
      (Utilities|IsValid (Variables|Initial|GetInitPart)
        (:Is%20Valid
          (CallFunction|InitialAttach))))))

(fn SlotMatch
  (params (Array :type Array%20of%20Strings))
  (bind _array_element (Utilities|Array|ForEachLoopwithBreak Array :!label _label)
    (:LoopBody
      (bind _output_get (LocalVariables|SetTMatch (Utilities|Array|ContainsItem (Variables|Settings|GetSlots) _array_element)))
      (if _output_get
        (goto _label Break)))
    (:Completed
      (return (LocalVariables|GetTMatch)))))

(fn CheckRequiredSlots
  (for _array_element (Variables|Requirements|GetRequiredSlots)
    (if (not (CallFunction|IsActive _array_element))
      (return false)))
  (for _array_element_2 (Variables|Requirements|GetReverseRequiredSlots)
    (if (CallFunction|IsActive _array_element_2)
      (return false)))
  (return true))

(fn IsActive
  (return (Variables|Default|GetAttached)))

(fn IsBlocked
  (for _array_element (Variables|Blocking|GetBlockers)
    (if (CallFunction|IsBlocking _array_element)
      (return true)))
  (return false))

(fn IsBlocking
  (return (Variables|Default|GetAttached)))

(fn InitialAttach
  (bind _slots (Class|BIAttach|GetSlots(Message) (Variables|Initial|GetInitPart)))
  (bind _match (CallFunction|SlotMatch _slots))
  (if (and (CallFunction|CheckRequiredSlots) _match)
    (CallFunction|Attach (Variables|Initial|GetInitPart))
    (return true)
    (else
      (Development|PrintString "Initial slots don't match or initial requirements are not fulfilled" true true "(R=1.000000,G=0.289567,B=0.000000,A=1.000000)" 5.0)
      (Variables|Initial|SetInitPart 0))))