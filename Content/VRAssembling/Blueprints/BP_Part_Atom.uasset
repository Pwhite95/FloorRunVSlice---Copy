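; Grabbable atom part for VR assembly that can be pulled, picked up, dropped and snapped into slots.
; The construction script builds it from atomic number, isotope and extra electrons, scattering instanced protons and neutrons around a nucleus and electrons in flat, randomized rings.
; Its slot name derives from the atomic number.
; Attaching releases it from the motion controller pawn; pickup detaches it from its slot unless that slot is blocked.
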(event EventPull
  (params (Controller :type BP%20Motion%20Controller%20Object%20Reference))
  (if (not (Variables|Default|GetAttached))
    (CallFunction|BasicPullForce (Variables|Default|GetSphere) (Transformation|GetWorldLocation (Variables|/Game/VRAssembling/Blueprints/BP_MotionController.BP_MotionController_C|GetGrabSphere Controller)) 5e+02)))

(event EventDrop
  (Transformation|DetachFromActor "KeepWorld" "KeepWorld" "KeepWorld")
  (Physics|SetSimulatePhysics (Variables|Default|GetSphere) (Variables|Default|GetSimulatePhysics)))

(event EventAttach
  (params (Slot :type BP%20Slot%20Base%20Object%20Reference))
  (Variables|Default|SetSlotActor Slot)
  (Utilities|FlowControl|Sequence
    (:then_0
      (Utilities|IsValid (Actor|GetAttachParentActor)
        (:Is%20Valid
          (bind _asbp_motion_controller_pawn (Utilities|Casting|CastToBP_MotionControllerPawn (Game|Player|GetPlayerPawn 0)))
          (Default|DropHolo _asbp_motion_controller_pawn self))))
    (:then_1
      (Transformation|AttachActorToActor (Variables|Default|GetSlotActor) "None" "SnapToTarget" "SnapToTarget" "KeepWorld" true)
      (Variables|Default|SetAttached true))))

(fn ConstructionScript
  (bind _output_get (LocalVariables|SetElectronRadius (Math|Float|Max(Float) (Math|Conversions|ToFloat(Integer) (Variables|Default|GetAtomicNumber)) 8.0)))
  (LocalVariables|SetNucleusRadius (/ _output_get 1e+01))
  (Components|Sphere|SetSphereRadius (Variables|Default|GetSphere) (LocalVariables|GetElectronRadius) true)
  (Physics|SetSimulatePhysics (Variables|Default|GetSphere) (Variables|Default|GetSimulatePhysics))
  (for _index (range 1 (Variables|Default|GetAtomicNumber))
    (Components|InstancedStaticMesh|AddInstance (Variables|Default|GetProton) (Math|Transform|MakeTransform (* (Math|Random|RandomUnitVector) (LocalVariables|GetNucleusRadius)) "0, 0, 0" "0.020000,0.020000,0.020000")))
  (for _index_2 (range 1 (+ (Variables|Default|GetAtomicNumber) (Variables|Default|GetIsotope)))
    (Components|InstancedStaticMesh|AddInstance (Variables|Default|GetNeutron) (Math|Transform|MakeTransform (* (Math|Random|RandomUnitVector) (LocalVariables|GetNucleusRadius)) "0, 0, 0" "0.020000,0.020000,0.020000")))
  (for _index_3 (range 1 (+ (Variables|Default|GetAtomicNumber) (Variables|Default|GetExtraElectrons)))
    (Components|InstancedStaticMesh|AddInstance (Variables|Default|GetElectron) (Math|Transform|MakeTransform (* (* (Math|Random|RandomUnitVector) "1.000000,1.000000,0.000000") (Math|Float|Max(Float) (* (LocalVariables|GetElectronRadius) (/ (Math|Conversions|ToFloat(Integer) (Math|Random|RandomInteger (+ (/ (+ (Variables|Default|GetAtomicNumber) (Variables|Default|GetExtraElectrons)) 8) 1))) (Math|Float|Max(Float) (Math|Conversions|ToFloat(Integer) (/ (+ (Variables|Default|GetAtomicNumber) (Variables|Default|GetExtraElectrons)) 8)) 1.0))) 8.0)) "0, 0, 0" "0.020000,0.020000,0.020000")))
  (Variables|Default|SetSlot (Utilities|String|Append "Atom" (Utilities|String|ToString(Integer) (Variables|Default|GetAtomicNumber)))))

(fn GetSlots
  (return (Utilities|Array|MakeArray (Variables|Default|GetSlot))))

(fn IsAttached
  (return (Variables|Default|GetAttached)))

(fn Pickup
  (params (AttachTo :type Scene%20Component%20Object%20Reference) (Hand :type BP%20Motion%20Controller%20Object%20Reference))
  (Utilities|IsValid (Variables|Default|GetSlotActor)
    (:Is%20Valid
      (if (Default|IsBlocked (Variables|Default|GetSlotActor))
        (return false)
        (else
          _)))
    (:Is%20Not%20Valid
      _))
  (Physics|SetSimulatePhysics (Variables|Default|GetSphere) false)
  (Transformation|AttachComponentToComponent AttachTo "None" "KeepWorld" "KeepWorld" "KeepWorld" true)
  (Utilities|IsValid (Variables|Default|GetSlotActor)
    (:Is%20Valid
      (Default|Detach (Variables|Default|GetSlotActor))
      (Variables|Default|SetSlotActor 0)
      (Variables|Default|SetAttached false)
      (return true))
    (:Is%20Not%20Valid
      (return true))))