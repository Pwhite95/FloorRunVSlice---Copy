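; A holographic assembly slot for a part that is screwed in along the slot's forward axis.
; Screw rotates and advances the attached actor by speed, notifies sub-slots and listeners when fully screwed or unscrewed, and drops it when backed out, unless locked.
; The slot counts as active only when fully screwed, and blocks past a quarter of the travel.
; The construction script can preview the end position with a hologram mesh.
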(event EventDetach
  (|CallParentFunction)
  (Variables|Default|SetCurDistance 0.0)
  (Variables|Default|SetScrewed false))

(fn ConstructionScript
  (|CallParentFunction)
  (if (Variables|Holo|Screw|GetShowEndPositionHoloEditor)
    (Components|StaticMesh|SetStaticMesh (Variables|Default|GetHelper) (Variables|Default|GetHoloMesh))
    (Transformation|SetRelativeTransform (Variables|Default|GetHelper) (Variables|Default|GetHoloTransform) false false)
    (Transformation|AddRelativeLocation (Variables|Default|GetHelper) (Math|Vector|MakeVector (Variables|Screw|GetScrewDistance) 0.0 0.0) false false)
    (for _index (range 0 (- (Rendering|Material|GetNumMaterials (Variables|Default|GetHelper)) 1))
      (Rendering|Material|SetMaterial (Variables|Default|GetHelper) _index "/Game/VRAssembling/Materials/M_Blueprint_Inst_Light.M_Blueprint_Inst_Light"))
    (else
      (Components|DestroyComponent (Variables|Default|GetHelper)))))

(fn IsActive
  (return (and (Variables|Default|GetAttached) (Variables|Default|GetScrewed))))

(fn Screw
  (params (Speed :type Float%20%28single-precision%29))
  (if (> Speed 0.0)
    (if (not (Variables|Default|GetScrewed))
      (Transformation|AddActorLocalRotation (Variables|Default|GetAttachedActor) (* (Variables|Screw|GetRotation) Speed) false false)
      (Variables|Default|SetCurDistance (+ (Variables|Default|GetCurDistance) Speed))
      (Transformation|AddActorWorldOffset (Variables|Default|GetAttachedActor) (* (Transformation|GetActorForwardVector) Speed))
      (bind _output_get (Variables|Default|SetScrewed (>= (Variables|Default|GetCurDistance) (Variables|Screw|GetScrewDistance))))
      (if _output_get
        (Utilities|FlowControl|Sequence
          (:then_0
            (for _array_element (Variables|Default|GetSubMessage)
              (Default|SubAttached _array_element self)))
          (:then_1
            (for _array_element_2 (Variables|Default|GetEventListeners)
              (Class|BIEvent|Screwed(Message) _array_element_2 self))))))
    (elif (not (and (Variables|Default|GetScrewed) (Variables|Default|GetLockPart)))
      (Transformation|AddActorLocalRotation (Variables|Default|GetAttachedActor) (* (Variables|Screw|GetRotation) Speed) false false)
      (Variables|Default|SetCurDistance (+ (Variables|Default|GetCurDistance) Speed))
      (Transformation|AddActorWorldOffset (Variables|Default|GetAttachedActor) (* (Transformation|GetActorForwardVector) Speed))
      (Utilities|FlowControl|Sequence
        (:then_0
          (if (Variables|Default|GetScrewed)
            (Utilities|FlowControl|Sequence
              (:then_0
                (Variables|Default|SetScrewed false))
              (:then_1
                (for _array_element_3 (Variables|Default|GetEventListeners)
                  (Class|BIEvent|Unscrewed(Message) _array_element_3 self)))
              (:then_2
                (for _array_element_4 (Variables|Default|GetSubMessage)
                  (Default|SubDetached _array_element_4 self))))))
        (:then_1
          (if (<= (Variables|Default|GetCurDistance) 0.0)
            (Class|BIPickup|Drop(Message) (Variables|Default|GetAttachedActor))
            (CallFunction|Detach)))))))

(fn IsBlocking
  (return (> (Variables|Default|GetCurDistance) (/ (Variables|Screw|GetScrewDistance) 4.0))))

(fn IsBlocked
  (return (or (|CallParentFunction) (CallFunction|IsBlocking))))

(fn InitialAttach
  (bind _attached (|CallParentFunction))
  (if _attached
    (bind _output_get (Variables|Default|SetCurDistance (Variables|Initial|GetInitialScrewDistance)))
    (Transformation|SetActorLocation (Variables|Default|GetInitPart) (+ (* (Transformation|GetActorForwardVector) _output_get) (Transformation|GetActorLocation)) false false)
    (return true)))