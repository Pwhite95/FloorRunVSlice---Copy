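; BP_Button is a pressable button for the VRAssembling content that notifies an EventActor when pressed and released.
; Touch projects an incoming velocity onto the button's up vector to move its clamped travel, while Tick steadily returns it to rest.
; A Pressed latch sends PressedMessage once at full depth and ReleasedMessage once the button is fully back up.
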(event EventTick
  (params (DeltaSeconds :type Float%20%28single-precision%29))
  (bind _output_get (Variables|Default|SetPress (Math|Float|Clamp(Float) (+ (Variables|Default|GetPress) DeltaSeconds) -1.0 0.0)))
  (Transformation|SetRelativeLocation (Variables|Default|GetButton) (Math|Vector|MakeVector 0.0 0.0 _output_get) false false)
  (if (and (== (Variables|Default|GetPress) 0.0) (Variables|Default|GetPressed))
    (Variables|Default|SetPressed false)
    (Class|BIButton|Released(Message) (Variables|Default|GetEventActor))))

(event EventTouch
  (params (Vel :type Vector :default "0, 0, 0"))
  (bind _output_get (Variables|Default|SetPress (Math|Float|Clamp(Float) (+ (Variables|Default|GetPress) (Math|Vector|DotProduct (Math|Vector|GetUpVector (Variables|Default|GetButton)) Vel)) -1.0 0.0)))
  (Transformation|SetRelativeLocation (Variables|Default|GetButton) (Math|Vector|MakeVector 0.0 0.0 _output_get) false false)
  (Utilities|FlowControl|Sequence
    (:then_0
      (if (and (== (Variables|Default|GetPress) -1.0) (not (Variables|Default|GetPressed)))
        (Variables|Default|SetPressed true)
        (Class|BIButton|Pressed(Message) (Variables|Default|GetEventActor))))
    (:then_1
      (if (and (== (Variables|Default|GetPress) 0.0) (Variables|Default|GetPressed))
        (Variables|Default|SetPressed false)
        (Class|BIButton|Released(Message) (Variables|Default|GetEventActor))))))

(fn ConstructionScript)