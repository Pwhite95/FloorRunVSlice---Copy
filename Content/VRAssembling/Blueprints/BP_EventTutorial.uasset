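; BP_EventTutorial is a VR assembling Blueprint that uses a point light to give visual feedback on part interaction events.
; The Attached event turns the light on in white and Detached hides it.
; Pushed recolors the light green and Screwed recolors it blue, with no other logic in the graph or construction script.
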(event EventAttached
  (params (Slot :type BP%20Slot%20Base%20Object%20Reference))
  (Rendering|SetVisibility (Variables|Default|GetPointLight) true false)
  (Rendering|Components|Light|SetLightColor (Variables|Default|GetPointLight) "(R=1.000000,G=1.000000,B=1.000000,A=1.000000)" true))

(event EventDetached
  (params (Slot :type BP%20Slot%20Base%20Object%20Reference))
  (Rendering|SetVisibility (Variables|Default|GetPointLight) false false))

(event EventPushed
  (params (Slot :type BP%20Slot%20Base%20Object%20Reference))
  (Rendering|Components|Light|SetLightColor (Variables|Default|GetPointLight) "(R=0.000000,G=1.000000,B=0.065985,A=1.000000)" true))

(event EventScrewed
  (params (Slot :type BP%20Slot%20Base%20Object%20Reference))
  (Rendering|Components|Light|SetLightColor (Variables|Default|GetPointLight) "(R=0.000000,G=0.180923,B=1.000000,A=1.000000)" true))

(fn ConstructionScript)