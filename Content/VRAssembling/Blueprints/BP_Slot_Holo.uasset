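; VR assembly slot that shows a tinted hologram mesh marking where a part attaches.
; The construction script builds the hologram component with a dynamic material unless the Holo mode is Never.
; Attach hides it, while Detach and sub-slot changes refresh it according to the mode and required-slot checks.
; Pickup and drop events count matching parts, showing the hologram while any are active, the slot is empty and requirements pass.
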(event Custom|CheckHolo
  (if (not (Variables|Default|GetAttached))
    (Rendering|SetVisibility (Variables|Holo|GetHoloComp) (CallFunction|CheckRequiredSlots) false)))

(event Custom|DropHolo
  (params (Part :type Actor%20Object%20Reference))
  (bind _slots (Class|BIAttach|GetSlots(Message) Part))
  (bind _match (CallFunction|SlotMatch _slots))
  (if _match
    (Math|Integer|DecrementInt (Variables|Default|GetHoloActive)
      (:%20%20
        (Rendering|SetVisibility (Variables|Holo|GetHoloComp) (Math|Boolean|ANDBoolean (> (Variables|Default|GetHoloActive) 0) (not (Variables|Default|GetAttached)) (CallFunction|CheckRequiredSlots)) false)))))

(event Custom|PickupHolo
  (params (Part :type Actor%20Object%20Reference))
  (bind _slots (Class|BIAttach|GetSlots(Message) Part))
  (bind _match (CallFunction|SlotMatch _slots))
  (if _match
    (Math|Integer|IncrementInt (Variables|Default|GetHoloActive)
      (:%20%20
        (Rendering|SetVisibility (Variables|Holo|GetHoloComp) (Math|Boolean|ANDBoolean (> (Variables|Default|GetHoloActive) 0) (not (Variables|Default|GetAttached)) (CallFunction|CheckRequiredSlots)) false)))))

(event EventBeginPlay
  (|CallParentFunction)
  (if (Utilities|Enum|NotEqual(Enum) (Variables|Holo|GetHolo) "NewEnumerator0")
    (Rendering|SetVisibility (Variables|Holo|GetHoloComp) (and (not (Utilities|IsValid (Variables|Default|GetInitPart))) (Utilities|Enum|Equal(Enum) (Variables|Holo|GetHolo) "NewEnumerator2")) false)))

(event EventSubAttached
  (params (Slot :type BP%20Slot%20Base%20Object%20Reference))
  (|CallParentFunction Slot)
  (if (Utilities|Enum|Equal(Enum) (Variables|Holo|GetHolo) "NewEnumerator3")
    (CallFunction|CheckHolo)))

(event EventSubDetached
  (params (Slot :type BP%20Slot%20Base%20Object%20Reference))
  (|CallParentFunction Slot)
  (if (Utilities|Enum|Equal(Enum) (Variables|Holo|GetHolo) "NewEnumerator3")
    (CallFunction|CheckHolo)))

(event EventDetach
  (|CallParentFunction)
  (switch Utilities|FlowControl|Switch|SwitchonE_Holo (Variables|Holo|GetHolo)
    (:NewEnumerator3
      (CallFunction|CheckHolo))
    (:NewEnumerator2
      (if true
        (Rendering|SetVisibility (Variables|Holo|GetHoloComp) true false)))))

(event EventAttach
  (params (AttachedActor :type Actor%20Object%20Reference))
  (|CallParentFunction AttachedActor)
  (if (Utilities|Enum|NotEqual(Enum) (Variables|Holo|GetHolo) "NewEnumerator0")
    (Rendering|SetVisibility (Variables|Holo|GetHoloComp) false false)))

(fn ConstructionScript
  (|CallParentFunction)
  (if (Utilities|Enum|NotEqual(Enum) (Variables|Holo|GetHolo) "NewEnumerator0")
    (bind _returnvalue (AddComponent|AddStaticMeshComponent false (Variables|Holo|GetHoloTransform)))
    (bind _output_get (Variables|Holo|SetHoloComp _returnvalue))
    (Components|StaticMesh|SetStaticMesh _output_get (Variables|Holo|GetHoloMesh))
    (bind _returnvalue_2 (Rendering|Material|CreateDynamicMaterialInstance "/Game/VRAssembling/Materials/M_Blueprint_Inst.M_Blueprint_Inst" "None" :!class /Script/Engine.KismetMaterialLibrary))
    (bind _output_get_2 (LocalVariables|SetMaterial _returnvalue_2))
    (Rendering|Material|SetVectorParameterValue _output_get_2 "Color" (Variables|Holo|GetHoloTint) :!class /Script/Engine.MaterialInstanceDynamic)
    (for _index (range 0 (- (Rendering|Material|GetNumMaterials (Variables|Holo|GetHoloComp)) 1))
      (Rendering|Material|SetMaterial (Variables|Holo|GetHoloComp) _index (LocalVariables|GetMaterial))
      (Rendering|SetVisibility (Variables|Holo|GetHoloComp) (and (Utilities|Enum|NotEqual(Enum) (Variables|Holo|GetHolo) "NewEnumerator0") (not (Utilities|IsValid (Variables|Default|GetInitPart)))) false))))