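; VR assembly slot variant in which an attached part must be pushed along a target vector before the slot counts as active.
; Touch moves the part by the velocity projected onto that axis, capped by remaining distance, then notifies sub-slots and listeners on arrival.
; An optional stretched hologram shows the push direction while pushing is pending.
; The construction script can also preview the end position, and initial parts can start partly pushed.
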(event Custom|Touch
  (params (Vel :type Vector))
  (bind _returnvalue (Transformation|GetActorLocation))
  (bind _pushtarget (Variables|Push|GetPushTarget))
  (bind _pushtarget_2 (Variables|Push|GetPushTarget))
  (bind _attachedactor (Variables|Default|GetAttachedActor))
  (bind _returnvalue_2 (Transformation|GetActorLocation _attachedactor))
  (bind _returnvalue_3 (Math|Vector|Normalize _pushtarget))
  (bind _returnvalue_4 (+ _pushtarget_2 _returnvalue))
  (bind _returnvalue_5 (Math|Vector|Distance(Vector) _returnvalue_4 _returnvalue_2))
  (if (and (Variables|Default|GetAttached) (not (Variables|Default|GetPushed)))
    (Transformation|AddActorWorldOffset (Variables|Default|GetAttachedActor) (* _returnvalue_3 (Math|Float|Min(Float) _returnvalue_5 (Math|Float|Max(Float) (Math|Vector|DotProduct Vel _returnvalue_3) 0.0))))
    (if (< _returnvalue_5 1.0)
      (Variables|Default|SetPushed true)
      (Utilities|FlowControl|Sequence
        (:then_0
          (for _array_element (Variables|Default|GetSubMessage)
            (Default|SubAttached _array_element self)))
        (:then_1
          (for _array_element_2 (Variables|Default|GetEventListeners)
            (Class|BIEvent|Pushed(Message) _array_element_2 self)))
        (:then_2
          (if (Variables|Holo|Push|GetShowPushHolo)
            (Rendering|SetVisibility (Variables|Default|GetStaticMesh) false false)))))))

(event EventBeginPlay
  (|CallParentFunction)
  (Variables|Push|SetPushTarget (Math|Vector|RotateVector (Variables|Push|GetPushTarget) (Transformation|GetActorRotation)))
  (if (Variables|Holo|Push|GetShowPushHolo)
    (Rendering|SetVisibility (Variables|Default|GetStaticMesh) false false)))

(event Collision|EventActorBeginOverlap
  (params (OtherActor :type Actor%20Object%20Reference)))

(event EventTick
  (params (DeltaSeconds :type Float%20%28single-precision%29)))

(event EventDetach
  (|CallParentFunction)
  (Variables|Default|SetPushed false)
  (if (Variables|Holo|Push|GetShowPushHolo)
    (Rendering|SetVisibility (Variables|Default|GetStaticMesh) false false)))

(event EventAttach
  (params (AttachedActor :type Actor%20Object%20Reference))
  (|CallParentFunction AttachedActor)
  (if (Variables|Holo|Push|GetShowPushHolo)
    (Rendering|SetVisibility (Variables|Default|GetStaticMesh) true false)))

(fn ConstructionScript
  (bind _pushtarget (Variables|Push|GetPushTarget))
  (|CallParentFunction)
  (Utilities|FlowControl|Sequence
    (:then_0
      (if (Variables|Holo|Push|GetShowPushHolo)
        (Transformation|SetRelativeTransform (Variables|Default|GetStaticMesh) (Math|Transform|MakeTransform (Variables|Holo|Push|GetPushHoloOffset) (Math|Conversions|RotationFromXVector _pushtarget) (Math|Vector|MakeVector (/ (Math|Vector|VectorLength _pushtarget) 1e+02) 0.1 0.1)) false false)
        (else
          (Components|DestroyComponent (Variables|Default|GetStaticMesh)))))
    (:then_1
      (if (Variables|Holo|Push|GetShowEndPositionHoloEditor)
        (Components|StaticMesh|SetStaticMesh (Variables|Default|GetHelper) (Variables|Default|GetHoloMesh))
        (Transformation|SetRelativeTransform (Variables|Default|GetHelper) (Variables|Default|GetHoloTransform) false false)
        (Transformation|AddRelativeLocation (Variables|Default|GetHelper) (Variables|Push|GetPushTarget) false false)
        (for _index (range 0 (- (Rendering|Material|GetNumMaterials (Variables|Default|GetHelper)) 1))
          (Rendering|Material|SetMaterial (Variables|Default|GetHelper) _index "/Game/VRAssembling/Materials/M_Blueprint_Inst_Light.M_Blueprint_Inst_Light"))
        (else
          (Components|DestroyComponent (Variables|Default|GetHelper)))))))

(fn IsActive
  (return (and (Variables|Default|GetAttached) (Variables|Default|GetPushed))))

(fn InitialAttach
  (bind _attached (|CallParentFunction))
  (if _attached
    (Transformation|SetActorLocation (Variables|Default|GetInitPart) (+ (Transformation|GetActorLocation) (* (Variables|Push|GetPushTarget) (Variables|Initial|GetInitialPush))) false false)
    (return true)))