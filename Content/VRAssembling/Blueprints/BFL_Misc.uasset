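; Blueprint function library of miscellaneous helpers for the VR assembling project.
; PrintVR repeats a debug string in a loop so it prints several times on screen.
; BasicPullForce draws a component toward a target: simulating bodies gain delta-time-scaled velocity with an upward lift term that grows with fast falls.
; Non-simulating components instead move by an unswept, scaled-down world offset.
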(fn PrintVR
  (params (InString :type String))
  (for _index (range 0 10)
    (Development|PrintString 0 InString true true "(R=0.000000,G=0.660000,B=1.000000,A=1.000000)" 5.0)))

(fn BasicPullForce
  (params (Comp :type Primitive%20Component%20Object%20Reference) (Target :type Vector) (Speed :type Float%20%28single-precision%29))
  (bind _returnvalue (Utilities|Time|GetWorldDeltaSeconds))
  (bind _returnvalue_2 (Transformation|GetWorldLocation Comp))
  (bind _returnvalue_3 (- Target _returnvalue_2))
  (bind _returnvalue_4 (Math|Vector|Normalize _returnvalue_3))
  (bind _returnvalue_5 (* _returnvalue_4 Speed))
  (if (Physics|IsSimulatingPhysics Comp "None")
    (Physics|SetPhysicsLinearVelocity Comp (* (+ (Math|Vector|MakeVector 0.0 0.0 (Math|Float|Max(Float) (* (.Z (Math|Vector|BreakVector (Transformation|GetComponentVelocity Comp))) -1.0) 1e+03)) _returnvalue_5) _returnvalue) true "None")
    (else
      (Transformation|AddWorldOffset Comp (* _returnvalue_5 (* _returnvalue 0.6)) false false))))