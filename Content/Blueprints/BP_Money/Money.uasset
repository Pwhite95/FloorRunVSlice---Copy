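; BP_Money is a money pickup that BP_MotionController can grab.
; Pickup disables physics on its Cube and attaches the root component to the given component, keeping its world transform.
; Drop detaches the actor, destroys it and plays a 2D explosion sound.
; Tick forces the Cube's relative roll to zero, leaving an unused roll-increment node disconnected.
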(event EventPickup
  (params (AttachTo :type Scene%20Component%20Object%20Reference))
  ;[1 1 1] Money Pick Up
  (Physics|SetSimulatePhysics (Variables|Default|GetCube) false)
  (Transformation|AttachComponentToComponent (VehicleSound|GetRootComponent) AttachTo "None" "KeepWorld" "KeepWorld" "KeepWorld" false))

(event EventTick
  (params (DeltaSeconds :type Float%20%28single-precision%29))
  (bind _cube (Variables|Default|GetCube))
  (bind _relativerotation (Variables|/Script/Engine.SceneComponent|GetRelativeRotation _cube))
  (Transformation|SetRelativeRotation _cube (Math|Rotator|MakeRotator 0.0 (.pitch _relativerotation) (.yaw _relativerotation)) false false))

(event EventDrop
  ;[1 1 1] Money Pick Up
  (Physics|SetSimulatePhysics (Variables|Default|GetCube) false)
  (Transformation|DetachFromActor "KeepWorld" "KeepWorld" "KeepWorld")
  (Actor|DestroyActor)
  (Audio|PlaySound2D "/Game/StarterContent/Audio/Explosion01.Explosion01" 1.0 1.0 0.0 0 0))

(fn ConstructionScript)